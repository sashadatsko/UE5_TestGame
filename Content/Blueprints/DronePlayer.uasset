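; Player-controlled drone character that flies, shoots projectiles and tracks health and ammo.
; Enhanced Input drives movement and look, while Shift and Space apply downward and upward velocity impulses for altitude.
; Left click spends ammo to spawn a projectile, and Tick refreshes the health and ammo texts alongside a HUD widget created at BeginPlay.
; Pickup-style functions add clamped ammo and health, and TakeDamage restarts the game when health runs out.
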(event Input|EnhancedActionEvents|EnhancedInputActionIA_Move
  (params (ActionValue :type Vector :default "0, 0, 0") (ElapsedSeconds :type Float%20%28double-precision%29) (TriggeredSeconds :type Float%20%28double-precision%29) (InputAction :type Input%20Action%20Object%20Reference :default "/Game/FirstPerson/Input/Actions/IA_Move.IA_Move"))
  (bind (_x _y) (Math|Vector|BreakVector ActionValue))
  (Pawn|Input|AddMovementInput (* (Transformation|GetActorForwardVector) _y) 1.0 false)
  (Pawn|Input|AddMovementInput (* (Transformation|GetActorRightVector) _x) 1.0 false))

(event Input|EnhancedActionEvents|EnhancedInputActionIA_Look
  (params (ActionValue :type Vector%202D%20Structure) (ElapsedSeconds :type Float%20%28double-precision%29) (TriggeredSeconds :type Float%20%28double-precision%29) (InputAction :type Input%20Action%20Object%20Reference :default "/Game/FirstPerson/Input/Actions/IA_Look.IA_Look"))
  (bind (_x _y) (Math|Vector2D|BreakVector2D ActionValue))
  (Pawn|Input|AddControllerPitchInput (* -1.0 _y))
  (Pawn|Input|AddControllerYawInput _x))

(event EventBeginPlay
  (Input|AddMappingContext (PlayerController|LocalPlayerSubsystems|GetEnhancedInputLocalPlayerSubsystem (Game|GetPlayerController 0)) "/Game/FirstPerson/Input/IMC_Default.IMC_Default" 0 "(bIgnoreAllPressedKeysUntilRelease=True,bForceImmediately=False,bNotifyUserSettings=False)")
  (bind _returnvalue (UserInterface|CreateWidget "/Game/Blueprints/HUD.HUD_C"))
  (UserInterface|Viewport|AddtoViewport _returnvalue 0))

(event EventTick
  (params (DeltaSeconds :type Float%20%28single-precision%29))
  (Rendering|Components|TextRender|SetText (Variables|Default|GetHeathText) (Utilities|Text|ToText(Integer) (Variables|Default|Gethealth)))
  (Rendering|Components|TextRender|SetText (Variables|Default|GetAmmoText) (Utilities|Text|ToText(Integer) (Variables|Default|Getammo))))

(event Input|MouseEvents|LeftMouseButton
  (params (Key :type Key%20Structure :default "None"))
  (:Pressed
    (if (> (Variables|Default|Getammo) 0)
      (Variables|Default|Setammo (- (Variables|Default|Getammo) 1))
      (Game|SpawnActorfromClass "/Game/Blueprints/Projectile2.Projectile2_C" (Transformation|GetWorldTransform (Variables|Default|GetProjectileSpawn)) "Undefined" "MultiplyWithRoot" 0 0))))

(event Input|KeyboardEvents|LeftShift
  (params (Key :type Key%20Structure :default "None"))
  (:Pressed
    (Physics|AddImpulse (Variables|Character|GetCharacterMovement) "0.000000,0.000000,-200.000000" true)))

(event Input|KeyboardEvents|SpaceBar
  (params (Key :type Key%20Structure :default "None"))
  (:Pressed
    (Physics|AddImpulse (Variables|Character|GetCharacterMovement) "0.000000,0.000000,200.000000" true)))

(fn ConstructionScript)

(fn AddAmmo
  (Variables|Default|Setammo (Math|Integer|Clamp(Integer) (+ 5 (Variables|Default|Getammo)) 0 20)))

(fn AddHealth
  (Variables|Default|Sethealth (Math|Integer|Clamp(Integer) (+ 20 (Variables|Default|Gethealth)) 0 100)))

(fn TakeDamage
  (if (> (Variables|Default|Gethealth) 20)
    (Variables|Default|Sethealth (- (Variables|Default|Gethealth) 20))
    (else
      (Default|RestartGame (.AsGame%20Mode (Utilities|Casting|CastToGameMode (Game|GetGameMode)))))))