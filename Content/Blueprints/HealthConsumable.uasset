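; Health pickup actor that restores health to the player's drone when touched.
; Tick spins the static mesh by a fixed step each frame, without delta-time scaling.
; When the Box overlaps the player-0 DronePlayer pawn, the actor destroys itself, calls AddHealth on the drone and prints its Health.
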(event OnComponentBeginOverlap(Box)
  (params (OverlappedComponent :type Primitive%20Component%20Object%20Reference) (OtherActor :type Actor%20Object%20Reference) (OtherComp :type Primitive%20Component%20Object%20Reference) (OtherBodyIndex :type Integer) (bFromSweep :type Boolean) (SweepResult :type Hit%20Result%20Structure%20%28by%20ref%29))
  (bind _returnvalue (Game|Player|GetPlayerPawn 0))
  (bind _asdrone_player (Utilities|Casting|CastToDronePlayer _returnvalue))
  (if (== OtherActor _asdrone_player)
    (Actor|DestroyActor)
    (Default|AddHealth _asdrone_player)
    (Development|PrintString (Utilities|String|ToString(Integer) (Variables|/Game/Blueprints/DronePlayer.DronePlayer_C|Gethealth _asdrone_player)))))

(event EventBeginPlay)

(event Collision|EventActorBeginOverlap
  (params (OtherActor :type Actor%20Object%20Reference)))

(event EventTick
  (params (DeltaSeconds :type Float%20%28single-precision%29))
  (Transformation|AddRelativeRotation (Variables|Default|GetStaticMesh) "0.000000,1.000000,0.000000" false false))

(fn ConstructionScript)