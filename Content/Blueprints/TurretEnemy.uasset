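; Turret enemy that lobs projectiles at the player and sinks as it takes hits.
; Within range on Tick, its light turns red and a random Delay paces shots spawned at ShootPos; out of range it turns green.
; Each blue-tinted Projectile2 gets an arced launch velocity toward the player from SuggestProjectileVelocityCustomArc.
; Sphere hits lower the actor and decrement Health, destroying it on a hit once Health is depleted.
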(event OnComponentHit(Sphere)
  (params (HitComponent :type Primitive%20Component%20Object%20Reference) (OtherActor :type Actor%20Object%20Reference) (OtherComp :type Primitive%20Component%20Object%20Reference) (NormalImpulse :type Vector :default "0, 0, 0") (Hit :type Hit%20Result%20Structure%20%28by%20ref%29))
  (bind _health (Variables|Default|Gethealth))
  (if (> _health 0)
    (Transformation|AddActorLocalOffset "0.000000,0.000000,-40.000000" false false)
    (Math|Integer|DecrementInt _health)
    (else
      (Actor|DestroyActor))))

(event EventTick
  (params (DeltaSeconds :type Float%20%28single-precision%29))
  (bind _returnvalue (Game|Player|GetPlayerPawn 0))
  (if (<= (Transformation|GetDistanceTo _returnvalue) 2e+03)
    (Rendering|Components|Light|SetLightColor (Variables|Default|GetPointLight) "(R=1.000000,G=0.000000,B=0.008842,A=1.000000)" false)
    (Utilities|FlowControl|Delay (Math|Random|RandomFloatinRange 0.5 2.0))
    (bind _returnvalue_2 (Game|SpawnActorfromClass "/Game/Blueprints/Projectile2.Projectile2_C" (Transformation|GetWorldTransform (Variables|Default|GetShootPos)) "Undefined" "MultiplyWithRoot" 0 0))
    (bind _outlaunchvelocity (Game|SuggestProjectileVelocityCustomArc (Transformation|GetActorLocation _returnvalue_2) (Transformation|GetActorLocation _returnvalue) 0.0 0.5))
    (Variables|/Script/Engine.MovementComponent|SetVelocity (Variables|/Game/Blueprints/Projectile2.Projectile2_C|GetProjectileMovement1 _returnvalue_2) _outlaunchvelocity)
    (Rendering|Material|SetMaterial (Variables|/Game/Blueprints/Projectile2.Projectile2_C|GetStaticMesh _returnvalue_2) 0 "/Game/Assets/Materials/MI_Solid_Blue.MI_Solid_Blue")
    (else
      (Rendering|Components|Light|SetLightColor (Variables|Default|GetPointLight) "(R=0.045745,G=1.000000,B=0.000000,A=1.000000)" false))))

(fn ConstructionScript)